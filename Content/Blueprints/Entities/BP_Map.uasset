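; BP_Map is an actor with two trigger boxes that work as a linked pair of teleporters for the player.
; When a BP_Player overlaps one box, it is teleported to the other box's world location with a zeroed rotation.
; A fixed sideways offset along world Y, opposite in sign for each destination, shifts the arrival point away from that box's center.
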(event OnComponentBeginOverlap(Box)
  (params (OverlappedComponent :type Primitive%20Component%20Object%20Reference) (OtherActor :type Actor%20Object%20Reference) (OtherComp :type Primitive%20Component%20Object%20Reference) (OtherBodyIndex :type Integer) (bFromSweep :type Boolean) (SweepResult :type Hit%20Result%20Structure%20%28by%20ref%29))
  (bind _asbp_player (Utilities|Casting|CastToBP_Player OtherActor))
  (Utilities|IsValid _asbp_player
    (:Is%20Valid
      (Transformation|Teleport _asbp_player (+ "0,-200.000000,0.000000" (Transformation|GetWorldLocation (Variables|Default|GetBox1))) "0, 0, 0"))))

(event OnComponentBeginOverlap(Box1)
  (params (OverlappedComponent :type Primitive%20Component%20Object%20Reference) (OtherActor :type Actor%20Object%20Reference) (OtherComp :type Primitive%20Component%20Object%20Reference) (OtherBodyIndex :type Integer) (bFromSweep :type Boolean) (SweepResult :type Hit%20Result%20Structure%20%28by%20ref%29))
  (bind _asbp_player (Utilities|Casting|CastToBP_Player OtherActor))
  (Utilities|IsValid _asbp_player
    (:Is%20Valid
      (Transformation|Teleport _asbp_player (+ "0,200.000000,0.000000" (Transformation|GetWorldLocation (Variables|Default|GetBox))) "0, 0, 0"))))

(event EventBeginPlay)

(event Collision|EventActorBeginOverlap
  (params (OtherActor :type Actor%20Object%20Reference)))

(event EventTick
  (params (DeltaSeconds :type Float%20%28single-precision%29)))

(fn ConstructionScript)