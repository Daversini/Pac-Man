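; BP_Player is the player character, which moves continuously in the last pressed of four directions and collects coins.
; Input presses store a Direction, and each Tick converts it to an axis value and adds forward or right movement input relative to control yaw, scaled by delta time and max walk speed.
; Capsule overlap with a BP_Coin destroys the coin and calls UpdateScore.
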(event OnComponentBeginOverlap(CapsuleComponent)
  (params (OverlappedComponent :type Primitive%20Component%20Object%20Reference) (OtherActor :type Actor%20Object%20Reference) (OtherComp :type Primitive%20Component%20Object%20Reference) (OtherBodyIndex :type Integer) (bFromSweep :type Boolean) (SweepResult :type Hit%20Result%20Structure%20%28by%20ref%29))
  (bind _asbp_coin (Utilities|Casting|CastToBP_Coin OtherActor))
  (Utilities|IsValid _asbp_coin
    (:Is%20Valid
      (Actor|DestroyActor _asbp_coin)
      (Default|CallUpdateScore))))

(event EventBeginPlay)

(event Collision|EventActorBeginOverlap
  (params (OtherActor :type Actor%20Object%20Reference)))

(event EventTick
  (params (DeltaSeconds :type Float%20%28single-precision%29))
  (bind _forward (CallFunction|SwitchonDirection))
  (CallFunction|Move _forward))

(event Input|ActionEvents|InputActionUp
  (params (Key :type Key%20Structure :default "None"))
  (:Pressed
    (Variables|Default|SetDirection "NewEnumerator0")))

(event Input|ActionEvents|InputActionDown
  (params (Key :type Key%20Structure :default "None"))
  (:Pressed
    (Variables|Default|SetDirection "NewEnumerator1")))

(event Input|ActionEvents|InputActionRight
  (params (Key :type Key%20Structure :default "None"))
  (:Pressed
    (Variables|Default|SetDirection "NewEnumerator2")))

(event Input|ActionEvents|InputActionLeft
  (params (Key :type Key%20Structure :default "None"))
  (:Pressed
    (Variables|Default|SetDirection "NewEnumerator3")))

(fn ConstructionScript)

(fn GetRotation
  (return (Math|Rotator|MakeRotator 0.0 0.0 (.yaw (Pawn|GetControlRotation :!class /Script/Engine.Pawn)))))

(fn SwitchonDirection
  (switch Utilities|FlowControl|Switch|SwitchonEnum_PlayerDirection (Variables|Default|GetDirection)
    (:NewEnumerator0
      (Variables|Default|SetForward%20Axis%20Value 1.0))
    (:NewEnumerator1
      (Variables|Default|SetForward%20Axis%20Value -1.0))
    (:NewEnumerator2
      (Variables|Default|SetRight%20Axis%20Value 1.0)
      (return false))
    (:NewEnumerator3
      (Variables|Default|SetRight%20Axis%20Value -1.0)
      (return false)))
  (return true))

(fn Move
  (params (Forward :type Boolean))
  (if Forward
    (Pawn|Input|AddMovementInput (Math|Vector|GetForwardVector (CallFunction|GetRotation)) (* (Variables|Default|GetForward%20Axis%20Value) (Utilities|Time|GetWorldDeltaSeconds) (Variables|/Script/Engine.CharacterMovementComponent|GetMaxWalkSpeed (Variables|Character|GetCharacterMovement))) false)
    (else
      (Pawn|Input|AddMovementInput (Math|Vector|GetRightVector (CallFunction|GetRotation)) (* (Variables|Default|GetRight%20Axis%20Value) (Utilities|Time|GetWorldDeltaSeconds) (Variables|/Script/Engine.CharacterMovementComponent|GetMaxWalkSpeed (Variables|Character|GetCharacterMovement))) false))))